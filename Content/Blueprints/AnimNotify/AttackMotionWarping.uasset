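; Motion warping notify state that steers a BladeCharacter's attack animation toward its auto target.
; On warp begin, a valid auto target feeds the character's FindMotionWarpingTargetTransform with angle, distance and reach-radius limits, and the result sets the "AttackTarget" warp target.
; On warp end, it removes that warp target.
; A debug arrow for the computed transform is present but unconnected.
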(fn `OnWarpBegin`
  (params (MotionWarpingComp :type "MotionWarpingComponent Object Reference") (Modifier :type "RootMotionModifier Object Reference"))
  (locals (AutoTarget :type "Character Object Reference"))
  (bind _asblade_character (cast `BladeCharacter` (`ActorComponent.GetOwner` MotionWarpingComp)))
  (bind _returnvalue (`BladeCharacter.GetAutoTarget` _asblade_character))
  (bind _output_get (set `local.AutoTarget` _returnvalue))
  (`/Engine/EditorBlueprintResources/StandardMacros.IsValid` _output_get
    (:`Is Valid`
      (`MotionWarpingComponent.AddOrUpdateWarpTargetFromTransform` (`BladeCharacter.MotionWarping` _asblade_character) "AttackTarget" (`BladeCharacter.FindMotionWarpingTargetTransform` _asblade_character _returnvalue (`self.MaxAngle`) (`self.MaxDistance`) (`self.ReachedRadius`))))))

(fn `OnWarpEnd`
  (params (MotionWarpingComp :type "MotionWarpingComponent Object Reference") (Modifier :type "RootMotionModifier Object Reference"))
  (`MotionWarpingComponent.RemoveWarpTarget` MotionWarpingComp "AttackTarget"))