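; WeaponBase is a weapon base Blueprint that resolves melee hits against other weapons and sword characters.
; Its OnHit event spawns a scaled-down block effect at the impact, aligned to the surface normal, when it strikes a BladeWeapon.
; Otherwise, a struck SwordCharacter takes fixed LightDamage point damage along the trace direction, credited to the weapon's owner, and has its name printed.
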(event `self.ReceiveBeginPlay`)

(event `OnHit`
  (params (HitComponent :type "PrimitiveComponent Object Reference") (OtherComponent :type "PrimitiveComponent Object Reference") (OtherActor :type "Actor Object Reference") (Hit :type "HitResult Structure (by ref)"))
  (bind (_bblockinghit _binitialoverlap _time _distance _location _impactpoint _normal _impactnormal _physmat _hitactor _hitcomponent _hitbonename _bonename _hititem _elementindex _faceindex _tracestart _traceend) (`GameplayStatics.BreakHitResult` Hit))
  (cast `BladeWeapon` OtherActor
    (:`then`
      (`GameplayStatics.SpawnEmitterAtLocation` "/Game/Effect/HitEffect/Particles/Effects_Block.Effects_Block" _impactpoint (`KismetMathLibrary.MakeRotFromZ` _impactnormal) (0.5 0.5 0.5)))
    (:`CastFailed`
      (bind _assword_character (cast `/Game/Characters/SwordMan/SwordCharacter` OtherActor))
      (`GameplayStatics.ApplyPointDamage` _assword_character 10.0 (`KismetMathLibrary.Normal` (- _traceend _tracestart)) Hit null (`self.GetOwner`) "/Game/Blueprints/DamageType/LightDamage.LightDamage_C")
      (`KismetSystemLibrary.PrintString` (`KismetSystemLibrary.GetDisplayName` _assword_character)))))

(fn `UserConstructionScript`)