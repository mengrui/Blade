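; Base player controller that lets the player swap the possessed pawn between character classes at runtime through debug keys.
; Three debug keys call ChangeCharacter with a fixed index into the CharacterClasses array.
; ChangeCharacter validates the index and pawn, records its transform, unpossesses and destroys it, then spawns and possesses the new class at that spot regardless of collision.
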(event EventBeginPlay)

(event EventTick
  (params (DeltaSeconds :type Float%20%28single-precision%29)))

(event Input|KeyboardEvents|DebugKey3
  (params (Key :type Key%20Structure :default "None") (ActionValue :type Input%20Action%20Value%20Structure))
  (:Pressed
    (CallFunction|ChangeCharacter 2)))

(event Input|KeyboardEvents|DebugKey1
  (params (Key :type Key%20Structure :default "None") (ActionValue :type Input%20Action%20Value%20Structure))
  (:Pressed
    (CallFunction|ChangeCharacter)))

(event Input|KeyboardEvents|DebugKey2
  (params (Key :type Key%20Structure :default "None") (ActionValue :type Input%20Action%20Value%20Structure))
  (:Pressed
    (CallFunction|ChangeCharacter 1)))

(fn ConstructionScript)

(fn ChangeCharacter
  (params (Index :type Integer))
  (bind _returnvalue (Pawn|GetControlledPawn))
  (bind _characterclasses (Variables|Default|GetCharacterClasses))
  (if (and (Utilities|Array|IsValidIndex _characterclasses Index) (Utilities|IsValid _returnvalue))
    (bind _output_get (LocalVariables|SetLastPawn _returnvalue))
    (bind _output_get_2 (LocalVariables|SetLastTransform (Transformation|GetActorTransform _output_get)))
    (Pawn|UnPossess)
    (Actor|DestroyActor _output_get)
    (bind _returnvalue_2 (Game|SpawnActorfromClass (Utilities|Array|Get(acopy) _characterclasses Index) _output_get_2 "AlwaysSpawn" "MultiplyWithRoot" 0 0))
    (Pawn|Possess _returnvalue_2)))