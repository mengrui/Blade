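; Test player controller that applies bullet damage to SilverCharacter actors under the mouse cursor on left click.
; Deprojects the cursor into the world and runs a debug-drawn line trace against PhysicsBody objects.
; A hit on a SilverCharacter receives point damage with the hit info and reversed ray direction, crediting the controller as instigator and its pawn as causer.
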(event `self.ReceiveTick`
  (params (DeltaSeconds :type "Float (single-precision)")))

(event `Key|LeftMouseButton`
  (params (Key :type "Key Structure"))
  (bind (_worldlocation _worlddirection) (`self.DeprojectMousePositionToWorld`))
  (:`Pressed`
    (bind _outhit (`KismetSystemLibrary.LineTraceSingleForObjects` :`Start` _worldlocation :`End` (+ _worldlocation (* _worlddirection 10000.0)) :`ObjectTypes` (`|MakeArray` "ObjectTypeQuery4" :!type "EObjectTypeQuery Enum") :`DrawDebugType` "ForDuration"))
    (bind _assilver_character (cast `/Game/Blueprints/Character/SilverCharacter` (`.HitActor` (`GameplayStatics.BreakHitResult` _outhit))))
    (`GameplayStatics.ApplyPointDamage` _assilver_character 1.0 (* _worlddirection -1.0) _outhit self (`self.K2_GetPawn`) "/Game/Blueprints/DamageType/BulletDamage.BulletDamage_C")))

(fn `UserConstructionScript`)