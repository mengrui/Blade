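; Behavior Tree task that repositions an AI pawn around its Blackboard target actor while keeping focus on it.
; It rotates the target-to-pawn direction by a random yaw up to 60 degrees either way, then picks a random distance between MinDistance and MaxDistance from the target.
; An AI move task heads there, finishing the task as failed on a rejected request and successful when movement ends.
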(event `self.ReceiveExecuteAI`
  (params (OwnerController :type "AIController Object Reference") (ControlledPawn :type "Pawn Object Reference"))
  (bind _asactor (cast `Actor` (`BTFunctionLibrary.GetBlackboardValueAsObject` (`self.TargetActor`))))
  (`AIController.K2_SetFocus` OwnerController _asactor)
  (bind _returnvalue (`Actor.K2_GetActorLocation` _asactor))
  (`AITask_MoveTo.AIMoveTo` OwnerController (+ _returnvalue (* (`KismetMathLibrary.Normal` (`KismetMathLibrary.GreaterGreater_VectorRotator` (- (`Actor.K2_GetActorLocation` ControlledPawn) _returnvalue) (`KismetMathLibrary.MakeRotator` 0.0 0.0 (`KismetMathLibrary.RandomFloatInRange` -60.0 60.0)))) (`KismetMathLibrary.RandomFloatInRange` (`self.MinDistance`) (`self.MaxDistance`)))) null
    (:`OnRequestFailed`
      (`self.FinishExecute` false))
    (:`OnMoveFinished`
      (`self.FinishExecute` true))))