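; Behavior tree service that finds the nearest BladeCharacterBase enemy for an AI pawn when search starts.
; It sphere-overlaps pawns filtered to BladeCharacter around the controlled pawn, ignoring itself, and writes each closer hit to the Target blackboard key.
; MinDist serves as both search radius and running closest distance, and is not reset within these graphs.
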(event `self.ReceiveSearchStartAI`
  (params (OwnerController :type "AIController Object Reference") (ControlledPawn :type "Pawn Object Reference"))
  (`self.FindNearestEnemy` ControlledPawn))

(fn `FindNearestEnemy`
  (params (OwnerPawn :type "Pawn Object Reference"))
  (locals (MinDist :type "Float (double-precision)" :default 3000.0) (NearTarget :type "Actor Object Reference"))
  (bind _outactors (`KismetSystemLibrary.SphereOverlapActors` (`Actor.K2_GetActorLocation` OwnerPawn) (`local.MinDist`) (`|MakeArray` "ObjectTypeQuery3" :!type "EObjectTypeQuery Enum") "/Script/Blade.BladeCharacter" (`|MakeArray` OwnerPawn :!type "Actor Object Reference")))
  (for _array_element _outactors
    (bind _asblade_character_base (cast `/Game/Blueprints/Character/BladeCharacterBase` _array_element))
    (bind _returnvalue (`Actor.GetDistanceTo` _asblade_character_base OwnerPawn))
    (if (< _returnvalue (`local.MinDist`))
      (set `local.MinDist` _returnvalue)
      (`BTFunctionLibrary.SetBlackboardValueAsObject` (`self.Target`) _asblade_character_base))))