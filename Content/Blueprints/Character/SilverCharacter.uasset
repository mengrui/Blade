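; SilverCharacter is a combat character Blueprint with target selection, physics-driven hit reactions, ragdoll knockdown and delayed death cleanup.
; Two attack inputs turn move direction into indices for neutral or four-way attacks.
; Hits apply delayed bone impulses while a timeline drives Physics Control strength; ragdolls recover after lying if still alive.
; Weapon hits add camera shake and curve-driven montage rate changes, while Gameplay Cameras sequences temporarily lock look input.
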(event OnComponentHit(CapsuleComponent)
  (params (HitComponent :type Primitive%20Component%20Object%20Reference) (OtherActor :type Actor%20Object%20Reference) (OtherComp :type Primitive%20Component%20Object%20Reference) (NormalImpulse :type Vector :default "0, 0, 0") (Hit :type Hit%20Result%20Structure%20%28by%20ref%29))
  (Utilities|Casting|CastTo OtherActor)
  (Variables|Default|SetHitNormal NormalImpulse))

(event Custom|OnWeaponHitOther
  (params (AnimRateCurve :type Curve%20Float%20Object%20Reference) (CameraShake :type Camera%20Shake%20Base%20Class%20Reference))
  (Camera|PlayWorldCameraShake CameraShake (Transformation|GetActorLocation) 1e+04 1e+05 1.0 true)
  (Class|TimelineComponent|SetFloatCurve (Variables|Default|GetTimelineAnimRate) AnimRateCurve "AnimPlayRate")
  (bind _animplayrate (Timeline|TimelineAnimRate PlayFromStart)
    (:Update
      (Animation|Montage|MontageSetPlayRate (CallFunction|GetAnimInstance) (Animation|GetCurrentMontage :!class /Script/Engine.Character) _animplayrate))))

(event Custom|PlayCameraSequence
  (params (CameraSequence :type Camera%20Animation%20Sequence%20Object%20Reference))
  (bind _returnvalue (Pawn|GetController))
  (bind _asplayer_controller (Utilities|Casting|CastToPlayerController _returnvalue))
  (Input|SetIgnoreLookInput _asplayer_controller true)
  (Pawn|SetControlRotation _returnvalue (Transformation|GetActorRotation))
  (bind _returnvalue_2 (CameraAnimation|PlayCameraAnimation (Subsystems|GetGameplayCamerasSubsystem) _asplayer_controller CameraSequence :!class /Script/GameplayCameras.GameplayCamerasSubsystem))
  (Variables|Default|SetCameraAnimHandle _returnvalue_2))

(event Custom|StopCameraAnimation
  (bind _asplayer_controller (Utilities|Casting|CastToPlayerController (Pawn|GetController)))
  (Input|SetIgnoreLookInput _asplayer_controller false)
  (CameraAnimation|StopCameraAnimation (Subsystems|GetGameplayCamerasSubsystem) _asplayer_controller (Variables|Default|GetCameraAnimHandle) :!class /Script/GameplayCameras.GameplayCamerasSubsystem))

(event Custom|FindTarget
  (bind _assilver_character (Utilities|Casting|CastTo (Variables|Default|GetSelectedTarget))
    (:then
      (Development|SetHiddeninGame (Variables|Default|GetTargetArrow _assilver_character) true false))
    (:CastFailed
      _))
  (CallFunction|SelectTarget)
  (bind _assilver_character_2 (Utilities|Casting|CastTo (Variables|Default|GetSelectedTarget)))
  (Development|SetHiddeninGame (Variables|Default|GetTargetArrow _assilver_character_2) false false))

(event Custom|CustomEvent)

(event Input|EnhancedActionEvents|EnhancedInputActionAttack0
  (params (ActionValue :type Boolean) (ElapsedSeconds :type Float%20%28double-precision%29) (TriggeredSeconds :type Float%20%28double-precision%29) (InputAction :type Input%20Action%20Object%20Reference :default "/Game/Blueprints/Input/Attack0.Attack0"))
  (bind _returnvalue (Input|EnhancedActionValues|GetMove))
  (bind _returnvalue_2 (Math|Vector|MakeVector (.x _returnvalue) (.y _returnvalue) 0.0))
  (:Triggered
    (CallFunction|Attack (select (Math|Vector|VectorIsZero _returnvalue_2) 0 (+ (Math|Float|Truncate (/ (Class|KismetMathLibrary|ClampAxis (+ (.yaw (Math|Conversions|RotationFromXVector _returnvalue_2)) 45.0)) 9e+01)) 1)))))

(event Input|EnhancedActionEvents|EnhancedInputActionAttack1
  (params (ActionValue :type Boolean) (ElapsedSeconds :type Float%20%28double-precision%29) (TriggeredSeconds :type Float%20%28double-precision%29) (InputAction :type Input%20Action%20Object%20Reference :default "/Game/Blueprints/Input/Attack1.Attack1"))
  (bind _returnvalue (Input|EnhancedActionValues|GetMove))
  (bind _returnvalue_2 (Math|Vector|MakeVector (.x _returnvalue) (.y _returnvalue) 0.0))
  (:Triggered
    (CallFunction|Attack (select (Math|Vector|VectorIsZero _returnvalue_2) 5 (+ (Math|Float|Truncate (/ (Class|KismetMathLibrary|ClampAxis (+ (.yaw (Math|Conversions|RotationFromXVector _returnvalue_2)) 45.0)) 9e+01)) 6)))))

(event EventBeginPlay
  (bind _mesh (Variables|Character|GetMesh))
  (Utilities|FlowControl|Sequence
    (:then_0
      (Class|PrimitiveComponent|SetLinearDamping _mesh 2.0)
      (Class|PrimitiveComponent|SetAngularDamping _mesh 1.0))
    (:then_1
      (bind _returnvalue (Game|ConstructObjectfromClass "/Game/UI/MainUI.MainUI_C"))
      (bind _output_get (Variables|Default|SetMainUI _returnvalue))
      (UserInterface|Viewport|AddtoViewport _output_get 0)
      (Variables|/Script/UMG.Widget|SetVisibility _output_get "Hidden"))))

(event Collision|EventActorBeginOverlap
  (params (OtherActor :type Actor%20Object%20Reference)))

(event EventTick
  (params (DeltaSeconds :type Float%20%28single-precision%29)))

(event EventOnPhysicsHit
  (params (Impulse :type Vector%20%28by%20ref%29 :default "0, 0, 0") (Location :type Vector%20%28by%20ref%29 :default "0, 0, 0") (BoneName :type Name%20%28by%20ref%29 :default "None"))
  (Variables|Default|SetbMoveAble false)
  (Utilities|FlowControl|Sequence
    (:then_0
      (bind _strength (Timeline|Timeline PlayFromStart)
        (:Update
          (Class|PhysicsControlComponent|SetControlMultipliers (Variables|Default|GetPhysicsControlComponent) (.names (Variables|Default|GetAllWorldSpaceControls)) (Utilities|Struct|MakePhysicsControlMultiplier (Math|Conversions|ToVector(Float) _strength) "1.000000,1.000000,1.000000" "1.000000,1.000000,1.000000" _strength 1.0 1.0) false))))
    (:then_1
      (Utilities|FlowControl|Delay 0.1)
      (Physics|AddImpulseatLocation (Variables|Character|GetMesh) Impulse Location BoneName))))

(event EventOnBecomeRagdoll
  (Utilities|FlowControl|Sequence
    (:then_0
      (Utilities|FlowControl|Delay (Variables|Default|GetLyingTime))
      (if (> (Variables|Default|GetHealth) 0.0)
        (CallFunction|SetRagdoll false)))
    (:then_1
      (bind _strength (Timeline|Timeline Stop)
        (:Update
          (Class|PhysicsControlComponent|SetControlMultipliers (Variables|Default|GetPhysicsControlComponent) (.names (Variables|Default|GetAllWorldSpaceControls)) (Utilities|Struct|MakePhysicsControlMultiplier (Math|Conversions|ToVector(Float) _strength) "1.000000,1.000000,1.000000" "1.000000,1.000000,1.000000" _strength 1.0 1.0) false))))))

(event EventOnDead
  (Utilities|FlowControl|Delay 1.0)
  (Actor|SetLifeSpan 5.0))

(event Input|KeyboardEvents|DebugKeyP
  (params (Key :type Key%20Structure :default "None") (ActionValue :type Input%20Action%20Value%20Structure))
  (:Pressed
    (if (CallFunction|IsRagdoll)
      (CallFunction|SetRagdoll false)
      (else
        (CallFunction|SetRagdoll true)))))

(event Input|KeyboardEvents|F
  (params (Key :type Key%20Structure :default "None")))

(fn ConstructionScript)