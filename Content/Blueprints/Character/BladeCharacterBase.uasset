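; Base Blueprint for blade-combat characters, handling physics hit reactions and ragdoll recovery.
; A hit event disables movement, plays a timeline scaling world-space Physics Control strength, and applies a bone impulse after a brief delay.
; Becoming a ragdoll stops that timeline and, after a lying time, exits ragdoll if health remains.
; Capsule hits from BladeWeapon actors record the normal impulse.
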(event `self.OnBecomeRagdoll`
  (bind _allworldspacecontrols_names (break `PhysicsControlNames` (`self.AllWorldSpaceControls`)))
  (`|ExecutionSequence`
    (:`then_0`
      (`KismetSystemLibrary.Delay` (`self.LyingTime`))
      (if (> (`self.Health`) 0.0)
        (`self.SetRagdoll` false)))
    (:`then_1`
      (bind (_direction _strength) (`Timeline|Timeline` :!via `Stop` :!label _label)
        (:`Update`
          (`PhysicsControlComponent.SetControlMultipliers` (`self.PhysicsControlComponent`) _allworldspacecontrols_names (make `PhysicsControlMultiplier` (`KismetMathLibrary.Conv_DoubleToVector` _strength) (1.0 1.0 1.0) (1.0 1.0 1.0) _strength) false))))))

(event `CustomEvent`
  (params (Impulse :type "Vector Structure (by ref)") (Location :type "Vector Structure (by ref)") (BoneName :type "Name (by ref)"))
  (set `self.bMoveAble` false)
  (`|ExecutionSequence`
    (:`then_0`
      (goto _label :!via `PlayFromStart`))
    (:`then_1`
      (`KismetSystemLibrary.Delay` 0.1)
      (`PrimitiveComponent.AddImpulseAtLocation` (`self.Mesh`) Impulse Location BoneName))))

(event `self.CapsuleComponent.OnComponentHit`
  (params (HitComponent :type "PrimitiveComponent Object Reference") (OtherActor :type "Actor Object Reference") (OtherComp :type "PrimitiveComponent Object Reference") (NormalImpulse :type "Vector Structure") (Hit :type "HitResult Structure (by ref)"))
  (cast `BladeWeapon` OtherActor)
  (set `self.HitNormal` NormalImpulse))

(fn `UserConstructionScript`)